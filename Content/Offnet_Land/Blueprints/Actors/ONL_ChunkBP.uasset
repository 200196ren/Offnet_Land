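; Voxel terrain chunk actor that builds its blocks on BeginPlay using size and noise settings from ONL_GameInstance.
; Initialize sets up Perlin fractal FastNoise and creates one instanced cube mesh component per material.
; GenerateBlocks samples noise at chunk-offset coordinates, placing only two surface blocks per column rather than filling it.
; AddBlock picks one of three material instances by fixed height thresholds and scales cubes to the block size.
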(event EventBeginPlay
  (CallFunction|Initialize)
  (CallFunction|GenerateBlocks))

(fn ConstructionScript)

(fn Initialize
  ;[1 1 1] Get the basic generate setting from ONL_GameInstance.
  (bind _asonl_game_instance (Utilities|Casting|CastToONL_GameInstance (Game|GetGameInstance)))
  (Variables|Basic|SetBlockSize (Variables|/Game/Offnet_Land/ONL_GameInstance.ONL_GameInstance_C|GetBlockSize _asonl_game_instance))
  (Variables|Basic|SetChunkHeight (Variables|/Game/Offnet_Land/ONL_GameInstance.ONL_GameInstance_C|GetChunkHeight _asonl_game_instance))
  (Variables|Basic|SetChunkSize (Variables|/Game/Offnet_Land/ONL_GameInstance.ONL_GameInstance_C|GetChunkSize _asonl_game_instance))
  ;[1 1 1] Set up the noise generator.
  (bind _returnvalue (Game|ConstructObjectfromClass "/Script/FastNoiseGenerator.FastNoiseWrapper"))
  (bind _output_get (Variables|AddBlock|SetFastNoiseWrapper _returnvalue))
  (Class|FastNoiseWrapper|SetupFastNoise _output_get "PerlinFractal" (Variables|/Game/Offnet_Land/ONL_GameInstance.ONL_GameInstance_C|GetNoiseSeed _asonl_game_instance) (Variables|/Game/Offnet_Land/ONL_GameInstance.ONL_GameInstance_C|GetNoiseFrequency _asonl_game_instance) "Hermite" "FBM" 3 2.0 0.5 0.45 "Euclidean" "CellValue")
  ;[1 1 1] Generate static meshes from materials.
  (for _array_element (Variables|Blocks|GetMaterials)
    (bind _returnvalue_2 (AddComponent|AddInstancedStaticMeshComponent false))
    (Components|StaticMesh|SetStaticMesh _returnvalue_2 "/Game/LevelPrototyping/Meshes/SM_Cube.SM_Cube")
    (Rendering|Material|SetMaterial _returnvalue_2 0 _array_element)
    (Utilities|Array|Add (Variables|Blocks|GetInstancedMeshes) _returnvalue_2)
    ;[1 1 1] Resize the list of Blocks
    (Utilities|Array|Resize (Variables|Blocks|GetBlocks) (* (Variables|Basic|GetChunkSize) (Variables|Basic|GetChunkSize) (Variables|Basic|GetChunkHeight)))))

(fn GenerateBlocks
  (bind _chunksize (Variables|Basic|GetChunkSize))
  (bind _chunksize_2 (Variables|Basic|GetChunkSize))
  (bind _chunkcoordinates (Variables|Basic|GetChunkCoordinates))
  (bind _returnvalue (- _chunksize_2 1))
  ;[1 1 1] Loops for (X, Y, Z)
  (for _index (range 0 _returnvalue)
    (Variables|AddBlock|SetX _index)
    (for _index_2 (range 0 _returnvalue)
      (Variables|AddBlock|SetY _index_2)
      (for _index_3 (range (Math|Float|Floor (* (+ (Class|FastNoiseWrapper|GetNoise2D (Variables|AddBlock|GetFastNoiseWrapper) (+ (* (.x _chunkcoordinates) _chunksize) (Variables|AddBlock|GetX)) (+ (* (.y _chunkcoordinates) _chunksize) (Variables|AddBlock|GetY))) 0.5) (Variables|Basic|GetChunkHeight))) (+ (Math|Float|Floor (* (+ (Class|FastNoiseWrapper|GetNoise2D (Variables|AddBlock|GetFastNoiseWrapper) (+ (* (.x _chunkcoordinates) _chunksize) (Variables|AddBlock|GetX)) (+ (* (.y _chunkcoordinates) _chunksize) (Variables|AddBlock|GetY))) 0.5) (Variables|Basic|GetChunkHeight))) 1))
        (Variables|AddBlock|SetZ _index_3)
        (CallFunction|AddBlock)))))

(fn AddBlock
  (bind _blocksize (Variables|Basic|GetBlockSize))
  (Components|InstancedStaticMesh|AddInstance (Utilities|Array|Get(acopy) (Variables|Blocks|GetInstancedMeshes) (Math|Integer|SelectInt (Math|Integer|SelectInt 0 1 (< (Variables|AddBlock|GetZ) 15)) 2 (< (Variables|AddBlock|GetZ) 27))) (Math|Transform|MakeTransform (Math|Vector|MakeVector (Math|Conversions|ToFloat(Integer) (* (Variables|AddBlock|GetX) _blocksize)) (Math|Conversions|ToFloat(Integer) (* (Variables|AddBlock|GetY) _blocksize)) (Math|Conversions|ToFloat(Integer) (* (Variables|AddBlock|GetZ) _blocksize))) "0, 0, 0" (* "1.000000,1.000000,1.000000" (/ (Math|Conversions|ToFloat(Integer) (Variables|Basic|GetBlockSize)) 100))) false))